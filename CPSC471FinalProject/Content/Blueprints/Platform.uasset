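; Platform is a ground segment actor that chains endless level generation and cleans up after itself.
; When the player overlaps its TriggerZone it calls the PlatformSpawner to spawn another platform, and overlapping its DestroyZone destroys it.
; Separate zones destroy Car and GreenTree actors that enter them.
; Hits on Cube and StaticMesh1 set a colliding car's Direction to opposite values, reversing its travel.
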(event `self.TriggerZone.OnComponentBeginOverlap`
  (params (OverlappedComponent :type "PrimitiveComponent Object Reference") (OtherActor :type "Actor Object Reference") (OtherComp :type "PrimitiveComponent Object Reference") (OtherBodyIndex :type Integer) (bFromSweep :type Boolean) (SweepResult :type "HitResult Structure (by ref)"))
  (cast `/Game/Blueprints/Player` OtherActor)
  (`/Game/Blueprints/PlatformSpawner.SpawnPlatformAtSpawnPoint` (`self.PlatformSpawner`)))

(event `self.DestroyZone.OnComponentBeginOverlap`
  (params (OverlappedComponent :type "PrimitiveComponent Object Reference") (OtherActor :type "Actor Object Reference") (OtherComp :type "PrimitiveComponent Object Reference") (OtherBodyIndex :type Integer) (bFromSweep :type Boolean) (SweepResult :type "HitResult Structure (by ref)"))
  (cast `/Game/Blueprints/Player` OtherActor)
  (`self.K2_DestroyActor`))

(event `self.CarDestroyZone.OnComponentBeginOverlap`
  (params (OverlappedComponent :type "PrimitiveComponent Object Reference") (OtherActor :type "Actor Object Reference") (OtherComp :type "PrimitiveComponent Object Reference") (OtherBodyIndex :type Integer) (bFromSweep :type Boolean) (SweepResult :type "HitResult Structure (by ref)"))
  (bind _ascar (cast `/Game/Blueprints/Car` OtherActor))
  (`self.K2_DestroyActor` _ascar))

(event `self.TreeDestroyZone.OnComponentBeginOverlap`
  (params (OverlappedComponent :type "PrimitiveComponent Object Reference") (OtherActor :type "Actor Object Reference") (OtherComp :type "PrimitiveComponent Object Reference") (OtherBodyIndex :type Integer) (bFromSweep :type Boolean) (SweepResult :type "HitResult Structure (by ref)"))
  (bind _asgreen_tree (cast `/Game/Blueprints/GreenTree` OtherActor))
  (`self.K2_DestroyActor` _asgreen_tree))

(event `self.Cube.OnComponentHit`
  (params (HitComponent :type "PrimitiveComponent Object Reference") (OtherActor :type "Actor Object Reference") (OtherComp :type "PrimitiveComponent Object Reference") (NormalImpulse :type "Vector Structure") (Hit :type "HitResult Structure (by ref)"))
  (bind _ascar (cast `/Game/Blueprints/Car` OtherActor))
  (set `/Game/Blueprints/Car.Direction` 200 _ascar))

(event `self.StaticMesh1.OnComponentHit`
  (params (HitComponent :type "PrimitiveComponent Object Reference") (OtherActor :type "Actor Object Reference") (OtherComp :type "PrimitiveComponent Object Reference") (NormalImpulse :type "Vector Structure") (Hit :type "HitResult Structure (by ref)"))
  (bind _ascar (cast `/Game/Blueprints/Car` OtherActor))
  (set `/Game/Blueprints/Car.Direction` -200 _ascar))

(fn `UserConstructionScript`)