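; Spawner actor that builds a chain of grass and road platforms starting beneath the player.
; On BeginPlay it clears existing platforms, cars and trees through nested loops, places a plain first platform, then chains more from the newest one's SpawnPoint.
; Each chained platform randomly gets grass with a tree or road with a car, offset randomly along X.
; Every platform receives a reference back to the spawner.
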(event `self.ReceiveBeginPlay`
  (`self.SpawnInitialPlatforms`))

(fn `SpawnInitialPlatforms`
  (bind _returnvalue (+ (`self.K2_GetActorLocation` (`GameplayStatics.GetPlayerPawn` 0)) (0.0 0.0 -150.0)))
  (`|ExecutionSequence`
    (:`then_0`
      (bind _outactors (`GameplayStatics.GetAllActorsOfClass` "/Game/Blueprints/Platform.Platform_C"))
      (for _array_element _outactors
        (`self.K2_DestroyActor` _array_element)
        (bind _outactors_2 (`GameplayStatics.GetAllActorsOfClass` "/Game/Blueprints/Car.Car_C"))
        (for _array_element_2 _outactors_2
          (`self.K2_DestroyActor` _array_element_2)
          (bind _outactors_3 (`GameplayStatics.GetAllActorsOfClass` "/Game/Blueprints/GreenTree.GreenTree_C"))
          (for _array_element_3 _outactors_3
            (`self.K2_DestroyActor` _array_element_3)))))
    (:`then_1`
      (`self.SpawnVeryFirstPlatform` _returnvalue)
      (for _ (range 13)
        (`/Engine/EditorBlueprintResources/StandardMacros.IsValid` (`self.NewestPlatform`)
          (:`Is Valid`
            (`self.SpawnPlatformAtSpawnPoint`))
          (:`Is Not Valid`
            (`self.SpawnPlatform` _returnvalue)))))))

(fn `SpawnPlatform`
  (params (`Spawn Location` :type "Vector Structure"))
  (locals (`Path picker` :type "StaticMesh Object Reference") (RandomInt :type Integer))
  (bind _newestplatform (`self.NewestPlatform`))
  (bind _returnvalue (+ (`KismetMathLibrary.MakeVector` (`KismetMathLibrary.RandomFloatInRange` -90.0 90.0) 0.0 1.5) `Spawn Location`))
  (bind _returnvalue_2 (`|SpawnActorFromClass` "/Game/Blueprints/Platform.Platform_C" (`KismetMathLibrary.MakeTransform` `Spawn Location`) "Undefined" "OverrideRootScale" null null))
  (bind _output_get (set `self.NewestPlatform` _returnvalue_2))
  (set `/Game/Blueprints/Platform.PlatformSpawner` self _output_get)
  (bind _output_get_2 (set `local.RandomInt` (`KismetMathLibrary.RandomIntegerInRange` 0 1)))
  (bind _output_get_3 (set `local.Path picker` (select `int` _output_get_2 :`0` "/Game/Blueprints/BigGrass2.BigGrass2" :`1` "/Game/Blueprints/Road.Road" :!type "StaticMesh Object Reference")))
  (`StaticMeshComponent.SetStaticMesh` (`/Game/Blueprints/Platform.BigGrass2` _newestplatform) _output_get_3)
  (`StaticMeshComponent.SetStaticMesh` (`/Game/Blueprints/Platform.BigGrass21` _newestplatform) _output_get_3)
  (`StaticMeshComponent.SetStaticMesh` (`/Game/Blueprints/Platform.StaticMesh` _newestplatform) _output_get_3)
  (`/Engine/EditorBlueprintResources/StandardMacros.CompareInt` _output_get_2
    (:`>`
      (`|SpawnActorFromClass` "/Game/Blueprints/Car.Car_C" (`KismetMathLibrary.MakeTransform` _returnvalue) "Undefined" "OverrideRootScale" null null))
    (:`==`
      (`|SpawnActorFromClass` "/Game/Blueprints/GreenTree.GreenTree_C" (`KismetMathLibrary.MakeTransform` _returnvalue) "Undefined" "OverrideRootScale" null null))))

(fn `SpawnPlatformAtSpawnPoint`
  (`self.SpawnPlatform` (`SceneComponent.K2_GetComponentLocation` (`/Game/Blueprints/Platform.SpawnPoint` (`self.NewestPlatform`)))))

(fn `SpawnVeryFirstPlatform`
  (params (`Spawn Location` :type "Vector Structure"))
  (locals (`Path picker` :type "StaticMesh Object Reference") (RandomInt :type Integer))
  (bind _returnvalue (`|SpawnActorFromClass` "/Game/Blueprints/Platform.Platform_C" (`KismetMathLibrary.MakeTransform` `Spawn Location`) "Undefined" "OverrideRootScale" null null))
  (bind _output_get (set `self.NewestPlatform` _returnvalue))
  (set `/Game/Blueprints/Platform.PlatformSpawner` self _output_get))

(fn `UserConstructionScript`)