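; Player pawn for a chicken hopping game, moved in discrete steps by the arrow keys.
; Key presses while grounded set flags that Tick turns into swept hop offsets and mesh rotations, under constant downward movement; Hit re-grounds it.
; The backward hop is disconnected, so Down only sets its flag.
; DisplayRestart shows the restart widget with UI input; RestartGame clears IsDead, restores game input and offsets the actor.
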(event `self.ReceiveHit`
  (params (MyComp :type "PrimitiveComponent Object Reference") (Other :type "Actor Object Reference") (OtherComp :type "PrimitiveComponent Object Reference") (bSelfMoved :type Boolean) (HitLocation :type "Vector Structure") (HitNormal :type "Vector Structure") (NormalImpulse :type "Vector Structure") (Hit :type "HitResult Structure (by ref)"))
  (set `self.IsOnGround` true))

(event `self.ReceiveBeginPlay`
  (bind _returnvalue (`|CreateWidget` "/Game/WBP_Restart.WBP_Restart_C"))
  (set `self.RestartWidget` _returnvalue))

(event `Key|Down`
  (params (Key :type "Key Structure"))
  (:`Pressed`
    (if (`self.IsOnGround`)
      (set `self.MoveBackward` true))))

(event `Key|Left`
  (params (Key :type "Key Structure"))
  (:`Pressed`
    (if (`self.IsOnGround`)
      (set `self.MoveLeft` true))))

(event `Key|Up`
  (params (Key :type "Key Structure"))
  (:`Pressed`
    (if (`self.IsOnGround`)
      (set `self.MoveForward` true))))

(event `Key|Right`
  (params (Key :type "Key Structure"))
  (:`Pressed`
    (if (`self.IsOnGround`)
      (set `self.MoveRight` true))))

(event `self.ReceiveTick`
  (params (DeltaSeconds :type "Float (single-precision)"))
  (if (not (`self.IsDead`))
    (`self.K2_AddActorLocalOffset` (* (0.0 0.0 -100.0) DeltaSeconds) true)
    (if (`self.MoveForward`)
      (`self.K2_AddActorLocalOffset` (0.0 20.0 20.0) true)
      (set `self.MoveForward` false)
      (set `self.IsOnGround` false)
      (`SceneComponent.K2_SetWorldRotation` (`self.Chicken`) (struct) false false)
      (elif (`self.MoveRight`)
        (`self.K2_AddActorLocalOffset` (-20.0 0.0 20.0) true)
        (set `self.MoveRight` false)
        (set `self.IsOnGround` false)
        (`SceneComponent.K2_SetWorldRotation` (`self.Chicken`) (struct :`Yaw` 90.0) false false)
        (elif (`self.MoveLeft`)
          (`self.K2_AddActorLocalOffset` (20.0 0.0 20.0) true)
          (set `self.MoveLeft` false)
          (set `self.IsOnGround` false)
          (`SceneComponent.K2_SetWorldRotation` (`self.Chicken`) (struct :`Yaw` -90.0) false false))))))

(fn `DisplayRestart`
  (bind _returnvalue (`GameplayStatics.GetPlayerController` 0))
  (`UserWidget.AddToViewport` (`self.RestartWidget`) 0)
  (`WidgetBlueprintLibrary.SetInputMode_UIOnlyEx` _returnvalue null)
  (set `PlayerController.bShowMouseCursor` true _returnvalue))

(fn `RestartGame`
  (bind _returnvalue (`GameplayStatics.GetPlayerController` 0))
  (set `self.IsDead` false)
  (`Widget.RemoveFromParent` (`self.RestartWidget`))
  (`WidgetBlueprintLibrary.SetInputMode_GameOnly` _returnvalue)
  (set `PlayerController.bShowMouseCursor` false _returnvalue)
  (`self.K2_AddActorWorldOffset` (0.0 -100.0 102.0)))

(fn `UserConstructionScript`)